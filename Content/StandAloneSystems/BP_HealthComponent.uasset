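; Health component that tracks current and max HP for its owning actor.
; BeginPlay sets starting HP, with a fallback max if none is set (current HP is then zero), and binds to the owner's OnTakeAnyDamage.
; Damage is negated into AdjustHealth, which clamps HP and fires one dispatcher at zero, another otherwise.
; A separate Death event sets IsDead; Tick and HPAdjust are empty.
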(event `self.ReceiveBeginPlay`
  (if (== (`self.MaxHP`) 0.0)
    ;[1 1 1] Need to find a way to set by the actor (any Actor)
    (set `self.MaxHP` 10.0)
    (set `self.CurrentHP` 0.0)
    (else
      (set `self.CurrentHP` (`self.MaxHP`))))
  (add `Actor.OnTakeAnyDamage` (`self.GetOwner`) (delegate `OnTakeAnyDamage_Event`)))

(event `OnTakeAnyDamage_Event`
  (params (DamagedActor :type "Actor Object Reference") (Damage :type "Float (single-precision)") (DamageType :type "DamageType Object Reference") (InstigatedBy :type "Controller Object Reference") (DamageCauser :type "Actor Object Reference"))
  (`self.AdjustHealth` (* Damage -1.0)))

(event `AdjustHealth`
  (params (HPAdjustment :type "Float (double-precision)"))
  (set `self.CurrentHP` (`KismetMathLibrary.FClamp` (+ (`self.CurrentHP`) HPAdjustment) 0.0 (`self.MaxHP`)))
  (if (== (`self.CurrentHP`) 0.0)
    (`self.Dispatch1`)
    (else
      (`self.Dispatch2`))))

(event `Death(HP)`
  (set `self.IsDead?` true))

(event `HPAdjust`)