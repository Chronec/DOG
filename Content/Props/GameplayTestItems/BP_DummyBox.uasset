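; BP_DummyBox is a gameplay test prop: a cube target with health that respawns after death.
; Its health component's dispatchers drive a red color flash and death.
; The flash resets by timer to grey, or to dark yellow when health is low.
; Death hides the cube and disables its collision, then a timer restores full HP, visibility and collision after RespawnTime.
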(event `Dispatch2_Event`
  (`MeshComponent.SetVectorParameterValueOnMaterials` (`self.Cube`) "Color" (1.0 0.0 0.0))
  (`KismetSystemLibrary.K2_SetTimerDelegate` (delegate `ResetColor`) 0.2))

(event `ResetColor`
  (if (> (`/Game/StandAloneSystems/BP_HealthComponent.CurrentHP` (`self.BP_HealthComponent`)) 6.0)
    (`MeshComponent.SetVectorParameterValueOnMaterials` (`self.Cube`) "Color" (0.8 0.8 0.8))
    (else
      (`MeshComponent.SetVectorParameterValueOnMaterials` (`self.Cube`) "Color" (0.4 0.4 0.0)))))

(event `self.ReceiveBeginPlay`
  (bind _bp_healthcomponent (`self.BP_HealthComponent`))
  (set `/Game/StandAloneSystems/BP_HealthComponent.MaxHP` (`self.Max HP`) (`self.BP_HealthComponent`))
  (add `/Game/StandAloneSystems/BP_HealthComponent.Dispatch1` _bp_healthcomponent (delegate `Death`))
  (add `/Game/StandAloneSystems/BP_HealthComponent.Dispatch2` _bp_healthcomponent (delegate `Dispatch2_Event`)))

(event `Death`
  ;[1 0.1212 0.07146] Death
  (`KismetSystemLibrary.PrintString` "Box Death" true false)
  (`self.Disappear`)
  (`KismetSystemLibrary.K2_SetTimerDelegate` (delegate `Respawn`) (`self.RespawnTime`)))

(event `Respawn`
  (bind _bp_healthcomponent (`self.BP_HealthComponent`))
  ;[0.3083 1 0.3895] Respawn
  (set `/Game/StandAloneSystems/BP_HealthComponent.CurrentHP` (`/Game/StandAloneSystems/BP_HealthComponent.MaxHP` _bp_healthcomponent) _bp_healthcomponent)
  (`self.ResetColor`)
  (`self.Reappear`)
  (`KismetSystemLibrary.PrintString` "DummyBox Respawn"))

(fn `Disappear`
  (`SceneComponent.SetVisibility` (`self.Cube`) false false)
  (`PrimitiveComponent.SetCollisionEnabled` (`self.Cube`) "NoCollision")
  (`PrimitiveComponent.SetCollisionResponseToChannel` (`self.Cube`) "ECC_Visibility" "ECR_Ignore"))

(fn `Reappear`
  (`SceneComponent.SetVisibility` (`self.Cube`) true false)
  (`PrimitiveComponent.SetCollisionEnabled` (`self.Cube`) "QueryAndPhysics")
  (`PrimitiveComponent.SetCollisionResponseToChannel` (`self.Cube`) "ECC_Visibility" "ECR_Block"))

(fn `UserConstructionScript`)