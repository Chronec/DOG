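; BP_DamageSpike is a gameplay test prop: a cone spike that damages any actor overlapping it, then temporarily disappears.
; On overlap it applies fixed damage to the other actor, then disables the cone's collision and hides it.
; A one-shot timer using RespawnTime then restores collision and visibility, re-arming the spike.
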(event `self.ReceiveActorBeginOverlap`
  (params (OtherActor :type "Actor Object Reference"))
  (`GameplayStatics.ApplyDamage` OtherActor 25.0)
  (`self.Die`)
  (`KismetSystemLibrary.K2_SetTimerDelegate` (delegate `Respawn`) (`self.RespawnTime`)))

(event `Respawn`
  (`PrimitiveComponent.SetCollisionEnabled` (`self.Cone`) "QueryAndPhysics")
  (`SceneComponent.SetVisibility` (`self.Cone`) true false))

(event `Die`
  (`PrimitiveComponent.SetCollisionEnabled` (`self.Cone`) "NoCollision")
  (`SceneComponent.SetVisibility` (`self.Cone`) false false))

(fn `UserConstructionScript`)