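; BP_DummyBox is a damageable dummy box prop that dies and respawns after a timed delay.
; AnyDamage subtracts from CurrentHP, prints it and flashes the cube's material red, then a timer restores a color chosen by remaining HP.
; Death fires only when HP equals exactly zero, hiding the cube and disabling its collision.
; A RespawnTime timer then restores max HP, color, visibility and collision.
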(event `Death`
  ;[1 0.1212 0.07146] Death
  (`self.Disappear`)
  (`KismetSystemLibrary.K2_SetTimerDelegate` (delegate `Respawn`) (`self.RespawnTime`)))

(event `self.ReceiveBeginPlay`
  (set `self.Current HP` (`self.Max HP`)))

(event `Respawn`
  ;[0.3083 1 0.3895] Respawn
  (set `self.Current HP` (`self.Max HP`))
  (`self.ResetColor`)
  (`self.Reappear`)
  (`KismetSystemLibrary.PrintString` "DummyBox Respawn"))

(event `self.ReceiveAnyDamage`
  (params (Damage :type "Float (single-precision)") (DamageType :type "DamageType Object Reference") (InstigatedBy :type "Controller Object Reference") (DamageCauser :type "Actor Object Reference"))
  ;[1 1 1] Taking damage
  (bind _output_get (set `self.Current HP` (- (`self.Current HP`) Damage)))
  (if (== (`self.Current HP`) 0.0)
    (`KismetSystemLibrary.PrintString` "Box Death" true false)
    (`self.Death`)
    (else
      (`KismetSystemLibrary.PrintString` (`KismetStringLibrary.Conv_DoubleToString` _output_get) true false)
      (`MeshComponent.SetVectorParameterValueOnMaterials` (`self.Cube`) "Color" (1.0 0.0 0.0))
      (`KismetSystemLibrary.K2_SetTimerDelegate` (delegate `ResetColor`) 0.2))))

(event `ResetColor`
  ;[1 1 1] Taking damage
  (if (> (`self.Current HP`) 6.0)
    (`MeshComponent.SetVectorParameterValueOnMaterials` (`self.Cube`) "Color" (0.8 0.8 0.8))
    (else
      (`MeshComponent.SetVectorParameterValueOnMaterials` (`self.Cube`) "Color" (0.4 0.4 0.0)))))

(fn `Disappear`
  (`SceneComponent.SetVisibility` (`self.Cube`) false false)
  (`PrimitiveComponent.SetCollisionEnabled` (`self.Cube`) "NoCollision")
  (`PrimitiveComponent.SetCollisionResponseToChannel` (`self.Cube`) "ECC_Visibility" "ECR_Ignore"))

(fn `Reappear`
  (`SceneComponent.SetVisibility` (`self.Cube`) true false)
  (`PrimitiveComponent.SetCollisionEnabled` (`self.Cube`) "QueryAndPhysics")
  (`PrimitiveComponent.SetCollisionResponseToChannel` (`self.Cube`) "ECC_Visibility" "ECR_Block"))

(fn `UserConstructionScript`)