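; BP_Melee gives the first-person character that owns it a melee attack triggered by the IA_Melee input.
; If off cooldown, it sphere-traces a short distance along the camera's forward vector from the owner's location, with debug drawing.
; Unless the hit component has the GameTraceChannel2 object type, it applies damage, prints valid hits and starts the cooldown, even on a miss.
; A timer event clears the cooldown.
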(event `CooldownEnded`
  (`KismetSystemLibrary.K2_ClearAndInvalidateTimerHandle` (`self.MeleeTimer`))
  (set `self.MeleeOnCooldown?` false))

(event `EnhancedInput|/Game/Character/FirstPerson/Input/Actions/Weapons/IA_Melee`
  (params (ActionValue :type Boolean) (ElapsedSeconds :type "Float (double-precision)") (TriggeredSeconds :type "Float (double-precision)") (InputAction :type "InputAction Object Reference" :default "/Game/Character/FirstPerson/Input/Actions/Weapons/IA_Melee.IA_Melee"))
  (bind _returnvalue (`self.GetOwner`))
  (bind _returnvalue_2 (`Actor.K2_GetActorLocation` _returnvalue))
  (:`Triggered`
    (if (not (`self.MeleeOnCooldown?`))
      (bind _asbp_first_person_character (cast `/Game/Character/FirstPerson/Blueprints/BP_FirstPersonCharacter` _returnvalue))
      (bind _outhit (`KismetSystemLibrary.SphereTraceSingle` _returnvalue_2 (+ _returnvalue_2 (* (`SceneComponent.GetForwardVector` (`/Game/Character/FirstPerson/Blueprints/BP_FirstPersonCharacter.FirstPersonCamera` _asbp_first_person_character)) 150.0)) 60.0 "TraceTypeQuery1" false (`|MakeArray` null :!type "Actor Object Reference") "ForDuration" true (struct :`R` 1.0 :`A` 1.0) (struct :`G` 1.0 :`A` 1.0) 3.0))
      (if (not (`|EnumEquality` (`PrimitiveComponent.GetCollisionObjectType` (`.HitComponent` (`GameplayStatics.BreakHitResult` _outhit))) "ECC_GameTraceChannel2"))
        (`GameplayStatics.ApplyDamage` (`.HitActor` (`GameplayStatics.BreakHitResult` _outhit)) 1.0)
        (`/Engine/EditorBlueprintResources/StandardMacros.IsValid` (`.HitActor` (`GameplayStatics.BreakHitResult` _outhit))
          (:`Is Valid`
            (`KismetSystemLibrary.PrintString` "Melee Hit"))
          (:`Is Not Valid`
            _))
        (set `self.MeleeOnCooldown?` true)
        (bind _returnvalue_3 (`KismetSystemLibrary.K2_SetTimerDelegate` (delegate `CooldownEnded`) (`self.MeleeCoodldown`)))
        (set `self.MeleeTimer` _returnvalue_3)))))