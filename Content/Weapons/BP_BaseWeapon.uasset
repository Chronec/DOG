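; Base weapon Blueprint that gives weapons shared setup and reload logic, with empty Shoot and Reload events.
; BeginPlay caches the first-person character and its player controller, then adds the weapon input mapping context.
; BaseReloadGun plays any given montage on the first-person mesh and uses its length to time Reloaded, which refills ammo and clears the reload flags.
; The base graph's own BaseReloadGun call is unconnected.
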(event `self.ReceiveBeginPlay`
  (`|ExecutionSequence`
    (:`then_0`
      ;[0 0.04614 1] Casting in the Base Blueprint one time so you never have to again
      (bind _asbp_first_person_character (cast `/Game/Character/FirstPerson/Blueprints/BP_FirstPersonCharacter` (`GameplayStatics.GetPlayerCharacter` 0)))
      (`/Engine/EditorBlueprintResources/StandardMacros.IsValid` _asbp_first_person_character
        (:`Is Valid`
          (bind _output_get (set `self.First Person Character` _asbp_first_person_character))
          (bind _asplayer_controller (cast `PlayerController` (`Pawn.GetController` _output_get)))
          (`/Engine/EditorBlueprintResources/StandardMacros.IsValid` (pcsubsystem `EnhancedInputLocalPlayerSubsystem` _asplayer_controller)
            (:`Is Valid`
              (set `self.PlayerController` _asplayer_controller)
              ;[0 1 0.106] Mapping Inputs On Base Weapon
              (message `EnhancedInputSubsystemInterface.AddMappingContext` (`self.PlayerController`) "/Game/Character/FirstPerson/Input/IMC_Weapons.IMC_Weapons" 0 (struct)))))))))

(event `Shoot_Weapon`)

(event `Reload_Weapon`)

(fn `BaseReloadGun`
  (params (GunMontage :type "AnimMontage Object Reference"))
  (bind _returnvalue (`AnimInstance.Montage_Play` (`SkeletalMeshComponent.GetAnimInstance` (`/Game/Character/FirstPerson/Blueprints/BP_FirstPersonCharacter.FirstPersonMesh` (`self.First Person Character`))) GunMontage 1.0 "MontageLength" 0.0 true))
  (bind _returnvalue_2 (`KismetSystemLibrary.K2_SetTimer` null "Reloaded" _returnvalue))
  (set `self.ReloadTimerHandle` _returnvalue_2)
  (set `self.IsReloding` true))

(fn `Reloaded`
  (set `self.IsReloding` false)
  (`KismetSystemLibrary.K2_ClearAndInvalidateTimerHandle` (`self.ReloadTimerHandle`))
  (set `self.AmmoCount` (`self.MaxAmmo`))
  (set `self.IsGunEmpty` false)
  (`KismetSystemLibrary.PrintString` "Reloading Complete"))

(fn `UserConstructionScript`)